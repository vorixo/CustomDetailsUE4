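; Flyable plane pawn that steers a physics-simulated mesh by setting its velocities directly.
; Pitch, yaw and roll axes become angular velocity vectors around the actor's own axes, summed and applied each Tick.
; Linear velocity is overwritten along the forward vector every Tick, with Left Shift switching to a faster speed.
; B toggles BugItOut, which replaces all three axis inputs with fixed values, forcing a constant tumble.
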(event `InputAxis|MoveUp`
  (params (AxisValue :type "Float (single-precision)"))
  ;[1 1 1] Input
  (set `self.Pitch_V` (* (`self.GetActorRightVector`) (* (select `bool` (`self.BugItOut`) :`false` AxisValue :`true` -0.8) (`self.PitchVel`)))))

(event `Key|B`
  (params (Key :type "Key Structure"))
  ;[1 1 1] Input
  (:`Pressed`
    (set `self.BugItOut` (not (`self.BugItOut`)))))

(event `InputAxis|MoveRight`
  (params (AxisValue :type "Float (single-precision)"))
  ;[1 1 1] Input
  (set `self.Right_V` (* (`self.GetActorUpVector`) (* (select `bool` (`self.BugItOut`) :`false` AxisValue :`true` 0.8) (`self.YawVel`)))))

(event `Key|LeftShift`
  (params (Key :type "Key Structure"))
  ;[1 1 1] Input
  (:`Pressed`
    (set `self.ForwardVel` 5000.0))
  (:`Released`
    (set `self.ForwardVel` 1500.0)))

(event `InputAxis|Roll`
  (params (AxisValue :type "Float (single-precision)"))
  ;[1 1 1] Input
  (set `self.Roll_V` (* (`self.GetActorForwardVector`) (* (select `bool` (`self.BugItOut`) :`false` AxisValue :`true` 0.8) (`self.RollVel`)))))

(event `self.ReceiveTick`
  (params (DeltaSeconds :type "Float (single-precision)"))
  ;[1 1 1] Tick
  (`parent.ReceiveTick` DeltaSeconds)
  (`PrimitiveComponent.SetPhysicsLinearVelocity` (`self.PlaneMesh`) (* (`self.GetActorForwardVector`) (`self.ForwardVel`)) false "None")
  (`PrimitiveComponent.SetPhysicsAngularVelocityInDegrees` (`self.PlaneMesh`) (+ (`self.Right_V`) (`self.Roll_V`) (`self.Pitch_V`)) false "None"))

(fn `UserConstructionScript`)